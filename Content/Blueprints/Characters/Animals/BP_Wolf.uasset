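; Wolf animal character Blueprint that supplies the wolf-specific death and attack animations.
; PlayAnimDeath plays the death animation once directly on the mesh, while PlayAttackAnimation plays the bite as an anim montage.
; It adds no other logic: BeginPlay, overlap and Tick are disabled stubs, and the construction script only calls the parent.
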(event EventBeginPlay
  (|CallParentFunction) ; This node is disabled and will not be called.\nDrag off pins to build functionality.
)

(event Collision|EventActorBeginOverlap
  (params (OtherActor :type Actor%20Object%20Reference))
  (|CallParentFunction OtherActor) ; This node is disabled and will not be called.\nDrag off pins to build functionality.
)

(event EventTick
  (params (DeltaSeconds :type Float%20%28single-precision%29))
  (|CallParentFunction DeltaSeconds) ; This node is disabled and will not be called.\nDrag off pins to build functionality.
)

(event EventPlayAnimDeath
  (Components|Animation|PlayAnimation (Variables|Character|GetMesh) "/Game/AnimalVarietyPack/Wolf/Animations/ANIM_Wolf_Death.ANIM_Wolf_Death" false))

(event EventPlayAttackAnimation
  (Animation|PlayAnimMontage "/Game/AnimalVarietyPack/Wolf/Animations/ANIM_Wolf_Bite_Montage.ANIM_Wolf_Bite_Montage" 1.0 "None"))

(fn ConstructionScript
  (|CallParentFunction))