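; Player character Blueprint for TinyRPG that handles interaction prompts, quest dialogs and the quest log.
; An interaction capsule attaches a prompt widget to overlapped quest or interactable components and removes it on end overlap.
; That prompt doubles as the current target: Interact follows its parent's owner to offer or turn in uncompleted quests and call InteractMessage, otherwise calling Interaction.
; DisplayQuestLog toggles the quest log widget on the game mode's HUD canvas.
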(event OnComponentBeginOverlap(InteractionCapsule)
  (params (OverlappedComponent :type Primitive%20Component%20Object%20Reference) (OtherActor :type Actor%20Object%20Reference) (OtherComp :type Primitive%20Component%20Object%20Reference) (OtherBodyIndex :type Integer) (bFromSweep :type Boolean) (SweepResult :type Hit%20Result%20Structure%20%28by%20ref%29))
  (Utilities|CheckforInteraction OtherActor
    (:HasQuest
      _)
    (:Interact
      _))
  (bind _returnvalue (AddComponent|AddWidgetComponent false))
  (bind _output_get (Variables|Default|SetInteractionMessage _returnvalue))
  (Transformation|AttachComponentToComponent _output_get OtherComp "None" "KeepRelative" "KeepRelative" "KeepRelative" true))

(event OnComponentEndOverlap(InteractionCapsule)
  (params (OverlappedComponent :type Primitive%20Component%20Object%20Reference) (OtherActor :type Actor%20Object%20Reference) (OtherComp :type Primitive%20Component%20Object%20Reference) (OtherBodyIndex :type Integer))
  (bind _interactionmessage (Variables|Default|GetInteractionMessage)
    (:then
      (Components|DestroyComponent _interactionmessage)
      (Variables|Default|SetInteractionMessage 0))
    (:else)))

(event EventBeginPlay)

(event Collision|EventActorBeginOverlap
  (params (OtherActor :type Actor%20Object%20Reference)))

(event EventTick
  (params (DeltaSeconds :type Float%20%28single-precision%29)))

(event Input|ActionEvents|InputActionDisplayQuestLog
  (params (Key :type Key%20Structure :default "None"))
  (:Pressed
    (bind _questlogui (Variables|Default|GetQuestLogUI)
      (:then
        (Widget|RemovefromParent _questlogui)
        (Variables|Default|SetQuestLogUI 0))
      (:else
        (bind _returnvalue (UserInterface|CreateWidget "/Game/Blueprints/QuestSystem/QuestUI/WBP_QuestLogUI.WBP_QuestLogUI_C"))
        (Variables|Default|SetQuestLogUI _returnvalue)
        (bind _asbp_tiny_rpggame_mode_base (Utilities|Casting|CastToBP_TinyRPGGameModeBase (Game|GetGameMode)))
        (bind _returnvalue_2 (Class|CanvasPanel|AddChildtoCanvas (Variables|/Game/Blueprints/BP_TinyRPGGameModeBase.BP_TinyRPGGameModeBase_C|GetHudCanvas _asbp_tiny_rpggame_mode_base) (Variables|Default|GetQuestLogUI)))
        (Class|CanvasPanelSlot|SetAnchors _returnvalue_2 (Utilities|Struct|MakeAnchors "(X=0.000000,Y=0.000000)" "(X=1.000000,Y=1.000000)"))))))

(event Input|ActionEvents|InputActionInteract
  (params (Key :type Key%20Structure :default "None"))
  (:Pressed
    (bind _interactionmessage (Variables|Default|GetInteractionMessage)
      (:then
        (bind _quest (Utilities|CheckforInteraction (Components|GetOwner (Transformation|GetAttachParent _interactionmessage)))
          (:HasQuest
            (if (not (Variables|/Script/TinyRPG.QuestBase|GetbIsCompleted _quest))
              (if (Utilities|Array|ContainsItem (Variables|/Script/TinyRPG.QuestLogComponent|GetQuests (Variables|Default|GetQuestLogComponent)) _quest)
                (Utilities|DisplayTurnin _quest
                  (:Out
                    (Class|InteractInterface|Interact(Message) (Components|GetOwner (Transformation|GetAttachParent _interactionmessage)))))
                (else
                  (Utilities|DisplayQuest _quest
                    (:Out
                      (Class|InteractInterface|Interact(Message) (Components|GetOwner (Transformation|GetAttachParent _interactionmessage)) :!label _label)))))
              (else
                (goto _label))))
          (:Interact
            (goto _label))))
      (:else
        (Class|TinyRPGCharacter|Interaction)))))

(fn ConstructionScript)